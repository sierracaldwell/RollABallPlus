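; BP_WinVolume is a trigger volume that wins the game when the player's pawn enters it.
; Any overlap with its Box spawns a particle system at the Cube's location and a win sound at the world origin, before the player check.
; If the overlapping actor is the player pawn, it calls Win on BallGameMode and starts a held camera fade-out.
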(event OnComponentBeginOverlap(Box)
  (params (OverlappedComponent :type Primitive%20Component%20Object%20Reference) (OtherActor :type Actor%20Object%20Reference) (OtherComp :type Primitive%20Component%20Object%20Reference) (OtherBodyIndex :type Integer) (bFromSweep :type Boolean) (SweepResult :type Hit%20Result%20Structure%20%28by%20ref%29))
  (Niagara|SpawnSystematLocation "/Game/_Game/Particles/PS_WinVolume.PS_WinVolume" (Transformation|GetWorldLocation (Variables|Default|GetCube)))
  (Audio|SpawnSoundatLocation "/Game/_Game/Audio/WinSFX_Cue.WinSFX_Cue" "0, 0, 0" "0, 0, 0" 1.0 1.0 0.0 0 0)
  (if (== OtherActor (Game|Player|GetPlayerPawn 0))
    (bind _asball_game_mode (Utilities|Casting|CastToBallGameMode (Game|GetGameMode)))
    (Default|Win _asball_game_mode)
    (CameraFades|StartCameraFade :self (Game|GetPlayerCameraManager 0) :ToAlpha 1.0 :Duration 3.0 :bHoldWhenFinished true)))

(event EventBeginPlay)

(event Collision|EventActorBeginOverlap
  (params (OtherActor :type Actor%20Object%20Reference)))

(event EventTick
  (params (DeltaSeconds :type Float%20%28single-precision%29)))

(fn ConstructionScript)